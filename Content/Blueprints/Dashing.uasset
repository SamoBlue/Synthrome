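; Dashing actor that carries the sci-fi hover car along a spline when the car overlaps its trigger box.
; The overlap opens a gate fed by Tick, which advances a distance by spline speed and delta time.
; A Cube follows the spline as a moving anchor, and the car teleports to its world transform.
; At the spline's end the car's linear velocity is zeroed and the gate closes; distance never resets.
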(event `self.Box.OnComponentBeginOverlap`
  (params (OverlappedComponent :type "PrimitiveComponent Object Reference") (OtherActor :type "Actor Object Reference") (OtherComp :type "PrimitiveComponent Object Reference") (OtherBodyIndex :type Integer) (bFromSweep :type Boolean) (SweepResult :type "HitResult Structure (by ref)"))
  (bind _cube (`self.Cube`))
  (bind (_returnvalue_location _returnvalue_rotation) (`KismetMathLibrary.BreakTransform` (`SplineComponent.GetTransformAtDistanceAlongSpline` (`self.Spline`) (`self.Distance`) "Local" false)))
  (bind _asbp_sci_fi_cyber_hover_car (cast `/Game/SciFiCyberHoverCar2/Blueprints/BP_SciFiCyberHoverCar` OtherActor))
  (goto _label :!via `Open`))

(event `self.ReceiveTick`
  (params (DeltaSeconds :type "Float (single-precision)"))
  (bind _cube (`self.Cube`))
  (bind (_returnvalue_location _returnvalue_rotation) (`KismetMathLibrary.BreakTransform` (`SplineComponent.GetTransformAtDistanceAlongSpline` (`self.Spline`) (`self.Distance`) "Local" false)))
  (`/Engine/EditorBlueprintResources/StandardMacros.Gate` true :!label _label
    (:`Exit`
      (set `self.Distance` (+ (* DeltaSeconds (`self.Spline Speed`)) (`self.Distance`)))
      (`SceneComponent.K2_SetRelativeTransform` (`self.Cube`) (`KismetMathLibrary.MakeTransform` _returnvalue_location _returnvalue_rotation) false false)
      (`self.K2_TeleportTo` (stale `self.Box.OnComponentBeginOverlap` _asbp_sci_fi_cyber_hover_car) (`SceneComponent.K2_GetComponentLocation` _cube) (`SceneComponent.K2_GetComponentRotation` _cube))
      (if (>= (`self.Distance`) (`SplineComponent.GetSplineLength` (`self.Spline`)))
        (`PrimitiveComponent.SetPhysicsLinearVelocity` (`WheeledVehiclePawn.Mesh` (stale `self.Box.OnComponentBeginOverlap` _asbp_sci_fi_cyber_hover_car)) (0.0 0.0 0.0) false "None")
        (goto _label :!via `Close`)))))

(fn `UserConstructionScript`)