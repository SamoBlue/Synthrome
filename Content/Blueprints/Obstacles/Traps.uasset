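; Moving obstacle trap that destroys any BP_SciFiCyberHoverCar touching its capsule.
; The construction script sets an InterpToMovement path between relative start and end locations, with duration taken from Timer.
; Tick re-randomizes Timer and activates the movement after random delays, without reapplying the duration.
; Overlap spawns an explosion at the car, zeroes its velocity and destroys it two seconds later, toggling input around the wait.
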(event `self.ReceiveTick`
  (params (DeltaSeconds :type "Float (single-precision)"))
  (bind _returnvalue (`KismetMathLibrary.RandomFloatInRange` 1.0 7.0))
  (set `self.Timer` _returnvalue)
  (`KismetSystemLibrary.Delay` (`KismetMathLibrary.RandomFloatInRange` 1.0 5.0))
  (`ActorComponent.Activate` (`self.InterpToMovement`) false)
  (`KismetSystemLibrary.Delay` _returnvalue))

(event `self.Capsule.OnComponentBeginOverlap`
  (params (OverlappedComponent :type "PrimitiveComponent Object Reference") (OtherActor :type "Actor Object Reference") (OtherComp :type "PrimitiveComponent Object Reference") (OtherBodyIndex :type Integer) (bFromSweep :type Boolean) (SweepResult :type "HitResult Structure (by ref)"))
  (bind _asbp_sci_fi_cyber_hover_car (cast `/Game/SciFiCyberHoverCar2/Blueprints/BP_SciFiCyberHoverCar` OtherActor))
  (`GameplayStatics.SpawnEmitterAtLocation` "/Game/StarterContent/Particles/P_Explosion.P_Explosion" (`self.K2_GetActorLocation` _asbp_sci_fi_cyber_hover_car) (struct) (10.0 10.0 10.0) false)
  (`self.DisableInput` null)
  (`PrimitiveComponent.SetPhysicsLinearVelocity` (`WheeledVehiclePawn.Mesh` _asbp_sci_fi_cyber_hover_car) (0.0 0.0 0.0) false "None")
  (`KismetSystemLibrary.Delay` 2.0)
  (`self.K2_DestroyActor` OtherActor)
  (`self.EnableInput` null))

(fn `UserConstructionScript`
  (bind _interptomovement (`self.InterpToMovement`))
  (set `InterpToMovementComponent.ControlPoints` (`|MakeArray` (make `InterpControlPoint` (`self.Start Location`)) (make `InterpControlPoint` (`self.End Location`))) _interptomovement)
  (set `InterpToMovementComponent.Duration` (`self.Timer`) _interptomovement))