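; Moving platform that starts travelling when a BP_SciFiCyberHoverCar begins overlapping its W component.
; The construction script builds InterpToMovement from relative StartLocation and EndLocation points, with Timer as duration.
; BeginPlay places W at the Plane's location, offset horizontally by Hitwall.
; A Tick-driven FlipFlop alternately plays and stops a Timeline that sets W's yaw, replaying after a delay when finished.
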(event `self.ReceiveTick`
  (params (DeltaSeconds :type "Float (single-precision)"))
  (`/Engine/EditorBlueprintResources/StandardMacros.FlipFlop`
    (:`A`
      (bind (_direction _newtrack_0) (`Timeline|Timeline` :!label _label)
        (:`Update`
          (`SceneComponent.K2_SetWorldRotation` (`self.w`) (`KismetMathLibrary.MakeRotator` 0.0 0.0 _newtrack_0) false false))
        (:`Finished`
          (`KismetSystemLibrary.Delay` 5.0)
          (goto _label :!via `PlayFromStart`))))
    (:`B`
      (goto _label :!via `Stop`))))

(event `self.w.OnComponentBeginOverlap`
  (params (OverlappedComponent :type "PrimitiveComponent Object Reference") (OtherActor :type "Actor Object Reference") (OtherComp :type "PrimitiveComponent Object Reference") (OtherBodyIndex :type Integer) (bFromSweep :type Boolean) (SweepResult :type "HitResult Structure (by ref)"))
  (cast `/Game/SciFiCyberHoverCar2/Blueprints/BP_SciFiCyberHoverCar` OtherActor)
  (`ActorComponent.Activate` (`self.InterpToMovement`) false))

(event `self.ReceiveBeginPlay`
  (bind (_x _y) (`KismetMathLibrary.BreakVector3f` (`self.Hitwall`)))
  (bind (_x_2 _y_2 _z) (`KismetMathLibrary.BreakVector3f` (`SceneComponent.K2_GetComponentLocation` (`self.Plane`))))
  (`SceneComponent.K2_SetWorldLocation` (`self.w`) (`KismetMathLibrary.MakeVector` (+ _x _x_2) (+ _y _y_2) _z) false false))

(fn `UserConstructionScript`
  (bind _interptomovement (`self.InterpToMovement`))
  (set `InterpToMovementComponent.ControlPoints` (`|MakeArray` (make `InterpControlPoint` (`self.Start Location`)) (make `InterpControlPoint` (`self.End Location`))) _interptomovement)
  (set `InterpToMovementComponent.Duration` (`self.Timer`) _interptomovement))