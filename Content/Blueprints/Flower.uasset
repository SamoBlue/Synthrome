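; Flower is an actor that creeps toward the player's BP_SciFiCyberHoverCar while the car is not grounded, and destroys itself once it is.
; Each Tick it teleports to an X/Y point interpolated between the car's mesh and its own Arrow component, keeping the Arrow's rotation.
; The blend sits very close to the Arrow and shifts slightly toward the car as forward speed rises, so the pull grows with speed.
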(event `self.ReceiveTick`
  (params (DeltaSeconds :type "Float (single-precision)"))
  (bind _arrow (`self.Arrow`))
  (bind _asbp_sci_fi_cyber_hover_car (cast `/Game/SciFiCyberHoverCar2/Blueprints/BP_SciFiCyberHoverCar` (`GameplayStatics.GetPlayerPawn` 0)))
  (if (`/Game/SciFiCyberHoverCar2/Blueprints/BP_SciFiCyberHoverCar.Grounded` _asbp_sci_fi_cyber_hover_car)
    (`self.K2_DestroyActor`)
    (else
      (bind (_returnvalue_x _returnvalue_y) (`KismetMathLibrary.BreakVector` (`KismetMathLibrary.VLerp` (`SceneComponent.K2_GetComponentLocation` (`WheeledVehiclePawn.Mesh` _asbp_sci_fi_cyber_hover_car)) (`SceneComponent.K2_GetComponentLocation` _arrow) (- 0.999 (/ (/ (`ChaosVehicleMovementComponent.GetForwardSpeed` (`/Game/SciFiCyberHoverCar2/Blueprints/BP_SciFiCyberHoverCar.ChaosWheeledVehicleMovement` _asbp_sci_fi_cyber_hover_car)) 1000000.0) 1.6)))))
      (`self.K2_TeleportTo` (`KismetMathLibrary.MakeVector` _returnvalue_x _returnvalue_y) (`SceneComponent.K2_GetComponentRotation` _arrow)))))

(fn `UserConstructionScript`)