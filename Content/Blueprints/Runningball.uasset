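; Running ball actor that launches a hidden physics component, W, when its WallHited event fires.
; WallHited blends the player's view to this actor, reveals W with physics on, then after a short delay adds velocity along Cube's forward vector.
; It then opens a Tick gate that teleports the actor to Cube's location with a fixed rotation every frame.
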(event `self.ReceiveTick`
  (params (DeltaSeconds :type "Float (single-precision)"))
  (`/Engine/EditorBlueprintResources/StandardMacros.Gate` true :!label _label
    (:`Exit`
      (`self.K2_TeleportTo` (`SceneComponent.K2_GetComponentLocation` (`self.Cube`)) (struct :`Yaw` 158.0)))))

(event `/Game/Blueprints/On_Off.WallHited`
  (bind _w (`self.w`))
  (`PlayerController.SetViewTargetWithBlend` (`GameplayStatics.GetPlayerController` 0) self 1.5 "VTBlend_Linear" 0.0 false)
  (`PrimitiveComponent.SetSimulatePhysics` _w true)
  (`SceneComponent.SetVisibility` _w true false)
  (`KismetSystemLibrary.Delay` 2.0)
  (`PrimitiveComponent.SetAllPhysicsLinearVelocity` (`self.w`) (* (`SceneComponent.GetForwardVector` (`self.Cube`)) 5500) true)
  (`|ExecutionSequence`
    (:`then_0`
      (goto _label :!via `Open`))))

(event `self.ReceiveBeginPlay`
  (`SceneComponent.SetVisibility` (`self.w`) false false))

(fn `UserConstructionScript`)