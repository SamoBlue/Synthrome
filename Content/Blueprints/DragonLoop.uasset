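; Dragon actor that builds a segmented dragon and flies it around a looping spline.
; Tick uses delays to spawn body segments up to a set length, then adds one tail and destroys segments in spawn order at a timed interval.
; A self-restarting Timeline, rate-scaled by a speed variable, places each segment along the spline, offset by array index and wrapped past the end.
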(event `Timeline`
  (bind _spline (`self.Spline`))
  (bind _distancealongs (`self.DistanceAlongS`))
  (bind _returnvalue (`SplineComponent.GetSplineLength` (`self.Spline`)))
  (bind (_direction _newtrack_0) (`Timeline|Timeline_0` :!via `PlayFromStart`)
    (:`Update`
      (for (_array_element _array_index) (`self.Actors`)
        (`/Engine/EditorBlueprintResources/StandardMacros.IsValid` _array_element
          (:`Is Valid`
            (bind _output_get (set `self.DistanceAlongS` (+ (`KismetMathLibrary.Lerp` 0.0 (`SplineComponent.GetSplineLength` (`self.Spline`)) _newtrack_0) (* _array_index (`self.Off sets`)))))
            (if (not (== (`SplineComponent.GetSplineLength` (`self.Spline`)) _output_get))
              (if (> _output_get _returnvalue)
                (set `self.DistanceAlongS` (- (`self.DistanceAlongS`) _returnvalue)))
              (`self.K2_SetActorLocationAndRotation` _array_element (`SplineComponent.GetLocationAtDistanceAlongSpline` _spline _distancealongs "World") (`SplineComponent.GetRotationAtDistanceAlongSpline` _spline _distancealongs "World") false false)
              (if true
                _))))))
    (:`Finished`
      (`self.Timeline`))))

(event `self.ReceiveBeginPlay`
  (`TimelineComponent.SetPlayRate` (`self.Timeline_0`) (/ 1.0 (`self.TimeL/DragonSpeed`)))
  (`self.Timeline`))

(event `self.ReceiveTick`
  (params (DeltaSeconds :type "Float (single-precision)"))
  (bind _first (`self.First`))
  (if (> (stale _returnvalue_3) (`self.Drgaon Length`))
    (`|ExecutionSequence`
      (:`then_0`
        (`KismetSystemLibrary.Delay` (`self.KillSpeed`))
        (if (not (> _first (+ (`self.Drgaon Length`) 2)))
          (`self.K2_DestroyActor` (`|GetArrayItem` (`self.Actors`) (`self.First`)))
          (set `self.First` (+ _first 1))))
      (:`then_1`
        (`/Engine/EditorBlueprintResources/StandardMacros.DoOnce` false
          (:`Completed`
            (bind _returnvalue (`|SpawnActorFromClass` "/Game/Blueprints/Dragon_tail.Dragon_tail_C" (`KismetMathLibrary.MakeTransform` (0.0 0.0 0.0)) "Undefined" "MultiplyWithRoot" null null))
            (`KismetArrayLibrary.Array_AddUnique` (`self.Actors`) _returnvalue)))))
    (else
      (`KismetSystemLibrary.Delay` (`self.SpawnSpeed`))
      (bind _returnvalue_2 (`|SpawnActorFromClass` "/Game/Blueprints/DragonBody.DragonBody_C" (`KismetMathLibrary.MakeTransform` (0.0 0.0 0.0)) "Undefined" "MultiplyWithRoot" null null))
      (bind _returnvalue_3 (`KismetArrayLibrary.Array_AddUnique` (`self.Actors`) _returnvalue_2)))))

(fn `UserConstructionScript`
  (bind _spline (`self.Spline`))
  (for (_array_element _array_index) (`self.Actors`)
    (`self.K2_SetActorLocationAndRotation` _array_element (`SplineComponent.GetLocationAtDistanceAlongSpline` _spline 0.0 "World") (`SplineComponent.GetRotationAtDistanceAlongSpline` _spline 0.0 "World") false false)))