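; Moving platform that carries the hover car between construction-set start and end points, once only.
; The first sphere overlap by the car activates InterpToMovement, disables car input and opens a Tick gate.
; While open, the gate teleports the car just above the sphere each frame, zeroing velocity and stepping yaw, so rotation is frame-rate dependent.
; A hardcoded delay, independent of the movement duration, restores input and closes the gate.
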(event `self.ReceiveTick`
  (params (DeltaSeconds :type "Float (single-precision)"))
  (bind (_returnvalue_x _returnvalue_y _returnvalue_z) (`KismetMathLibrary.BreakVector` (`SceneComponent.K2_GetComponentLocation` (`self.Sphere`))))
  (`/Engine/EditorBlueprintResources/StandardMacros.Gate` true :!label _label
    (:`Exit`
      (`self.K2_TeleportTo` (stale `self.Sphere.OnComponentBeginOverlap` _asbp_sci_fi_cyber_hover_car) (`KismetMathLibrary.MakeVector` _returnvalue_x _returnvalue_y (+ _returnvalue_z 10.0)) (`KismetMathLibrary.MakeRotator` 0.0 0.0 (`self.Dest Rotation X (Roll)`)))
      (set `self.Dest Rotation X (Roll)` (+ (`self.Dest Rotation X (Roll)`) -0.25))
      (`PrimitiveComponent.SetPhysicsLinearVelocity` (`WheeledVehiclePawn.Mesh` (stale `self.Sphere.OnComponentBeginOverlap` _asbp_sci_fi_cyber_hover_car)) (0.0 0.0 0.0) false "None"))))

(event `self.Sphere.OnComponentBeginOverlap`
  (params (OverlappedComponent :type "PrimitiveComponent Object Reference") (OtherActor :type "Actor Object Reference") (OtherComp :type "PrimitiveComponent Object Reference") (OtherBodyIndex :type Integer) (bFromSweep :type Boolean) (SweepResult :type "HitResult Structure (by ref)"))
  (`/Engine/EditorBlueprintResources/StandardMacros.DoOnce` false
    (:`Completed`
      (bind _asbp_sci_fi_cyber_hover_car (cast `/Game/SciFiCyberHoverCar2/Blueprints/BP_SciFiCyberHoverCar` OtherActor))
      (`ActorComponent.Activate` (`self.InterpToMovement`) false)
      (`self.DisableInput` _asbp_sci_fi_cyber_hover_car null)
      (`PrimitiveComponent.SetPhysicsLinearVelocity` (`WheeledVehiclePawn.Mesh` _asbp_sci_fi_cyber_hover_car) (0.0 0.0 0.0) false "None")
      (`|ExecutionSequence`
        (:`then_0`
          (goto _label :!via `Open`))
        (:`then_1`
          (`KismetSystemLibrary.Delay` 18.1)
          (`self.EnableInput` _asbp_sci_fi_cyber_hover_car null)
          (goto _label :!via `Close`))))))

(fn `UserConstructionScript`
  (bind _interptomovement (`self.InterpToMovement`))
  (set `InterpToMovementComponent.ControlPoints` (`|MakeArray` (make `InterpControlPoint` (`self.Start Location`)) (make `InterpControlPoint` (`self.End Location`))) _interptomovement)
  (set `InterpToMovementComponent.Duration` (`self.Timer`) _interptomovement))