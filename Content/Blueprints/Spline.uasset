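; Spline actor that moves a Cube component along its Spline component at a set speed.
; Each Tick advances a distance by SplineSpeed times delta time, then sets the cube's relative location and rotation from the spline's local-space transform at that distance.
; When Looped is true, the distance resets to zero once it exceeds the spline length, restarting the path from the beginning.
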(event `self.ReceiveTick`
  (params (DeltaSeconds :type "Float (single-precision)"))
  (bind (_returnvalue_location _returnvalue_rotation) (`KismetMathLibrary.BreakTransform` (`SplineComponent.GetTransformAtDistanceAlongSpline` (`self.Spline`) (`self.Distance`) "Local" false)))
  (set `self.Distance` (+ (* DeltaSeconds (`self.Spline Speed`)) (`self.Distance`)))
  (`SceneComponent.K2_SetRelativeTransform` (`self.Cube`) (`KismetMathLibrary.MakeTransform` _returnvalue_location _returnvalue_rotation) false false)
  (if (`self.Looped ?`)
    (if (> (`self.Distance`) (`SplineComponent.GetSplineLength` (`self.Spline`)))
      (set `self.Distance` 0.0))))

(fn `UserConstructionScript`)