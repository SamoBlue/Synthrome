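; Finishing platform Blueprint that sets off a celebratory spark sequence when the hover car reaches it.
; Its ten spark particle components are deactivated on BeginPlay.
; When a BP_SciFiCyberHoverCar overlaps the Box trigger, the sparks activate in pairs, staggered by short delays to form a cascading effect.
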(event `self.ReceiveBeginPlay`
  (`ActorComponent.Deactivate` (`self.P_Sparks8`))
  (`ActorComponent.Deactivate` (`self.P_Sparks7`))
  (`ActorComponent.Deactivate` (`self.P_Sparks6`))
  (`ActorComponent.Deactivate` (`self.P_Sparks9`))
  (`ActorComponent.Deactivate` (`self.P_Sparks4`))
  (`ActorComponent.Deactivate` (`self.P_Sparks`))
  (`ActorComponent.Deactivate` (`self.P_Sparks1`))
  (`ActorComponent.Deactivate` (`self.P_Sparks2`))
  (`ActorComponent.Deactivate` (`self.P_Sparks3`))
  (`ActorComponent.Deactivate` (`self.P_Sparks5`)))

(event `self.Box.OnComponentBeginOverlap`
  (params (OverlappedComponent :type "PrimitiveComponent Object Reference") (OtherActor :type "Actor Object Reference") (OtherComp :type "PrimitiveComponent Object Reference") (OtherBodyIndex :type Integer) (bFromSweep :type Boolean) (SweepResult :type "HitResult Structure (by ref)"))
  (cast `/Game/SciFiCyberHoverCar2/Blueprints/BP_SciFiCyberHoverCar` OtherActor)
  (`ActorComponent.Activate` (`self.P_Sparks1`) false)
  (`ActorComponent.Activate` (`self.P_Sparks`) false)
  (`KismetSystemLibrary.Delay` 0.5)
  (`ActorComponent.Activate` (`self.P_Sparks2`) false)
  (`ActorComponent.Activate` (`self.P_Sparks3`) false)
  (`KismetSystemLibrary.Delay` 0.5)
  (`ActorComponent.Activate` (`self.P_Sparks4`) false)
  (`ActorComponent.Activate` (`self.P_Sparks5`) false)
  (`KismetSystemLibrary.Delay` 0.5)
  (`ActorComponent.Activate` (`self.P_Sparks6`) false)
  (`ActorComponent.Activate` (`self.P_Sparks7`) false)
  (`KismetSystemLibrary.Delay` 0.5)
  (`ActorComponent.Activate` (`self.P_Sparks9`) false)
  (`ActorComponent.Activate` (`self.P_Sparks8`) false))

(fn `UserConstructionScript`)