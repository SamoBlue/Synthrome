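; PickUps is a collectible actor that rewards the player's hover car when touched.
; Its sphere overlap casts to BP_SciFiCyberHoverCar, calls AddNitro and increments the car's pickup count.
; It also adds points from a flat bonus plus a share of the car's forward speed, then destroys itself.
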(event `self.Sphere.OnComponentBeginOverlap`
  (params (OverlappedComponent :type "PrimitiveComponent Object Reference") (OtherActor :type "Actor Object Reference") (OtherComp :type "PrimitiveComponent Object Reference") (OtherBodyIndex :type Integer) (bFromSweep :type Boolean) (SweepResult :type "HitResult Structure (by ref)"))
  (bind _asbp_sci_fi_cyber_hover_car (cast `/Game/SciFiCyberHoverCar2/Blueprints/BP_SciFiCyberHoverCar` OtherActor))
  (`/Game/SciFiCyberHoverCar2/Blueprints/BP_SciFiCyberHoverCar.Add Nitro` _asbp_sci_fi_cyber_hover_car)
  (set `/Game/SciFiCyberHoverCar2/Blueprints/BP_SciFiCyberHoverCar.Pickups` (+ (`/Game/SciFiCyberHoverCar2/Blueprints/BP_SciFiCyberHoverCar.Pickups` _asbp_sci_fi_cyber_hover_car) 1.0) _asbp_sci_fi_cyber_hover_car)
  (set `/Game/SciFiCyberHoverCar2/Blueprints/BP_SciFiCyberHoverCar.Points` (+ (`/Game/SciFiCyberHoverCar2/Blueprints/BP_SciFiCyberHoverCar.Points` _asbp_sci_fi_cyber_hover_car) (+ (/ (`ChaosVehicleMovementComponent.GetForwardSpeed` (`WheeledVehiclePawn.VehicleMovementComponent` _asbp_sci_fi_cyber_hover_car)) 10.0) 200.0)) _asbp_sci_fi_cyber_hover_car)
  (`self.K2_DestroyActor`))

(fn `UserConstructionScript`)