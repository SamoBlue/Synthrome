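; Hitwall is a trigger actor that reports when a BP_SciFiCyberHoverCar runs into its box volume.
; On begin overlap it filters for the hover car by cast, then calls WallHitedMessage on five separately referenced Controlled objects.
; The response to the hit is left entirely to those objects, and other overlapping actors are ignored.
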(event `self.Box.OnComponentBeginOverlap`
  (params (OverlappedComponent :type "PrimitiveComponent Object Reference") (OtherActor :type "Actor Object Reference") (OtherComp :type "PrimitiveComponent Object Reference") (OtherBodyIndex :type Integer) (bFromSweep :type Boolean) (SweepResult :type "HitResult Structure (by ref)"))
  (cast `/Game/SciFiCyberHoverCar2/Blueprints/BP_SciFiCyberHoverCar` OtherActor)
  (message `/Game/Blueprints/On_Off.WallHited` (`self.Controlled_1`))
  (message `/Game/Blueprints/On_Off.WallHited` (`self.Controlled_2`))
  (message `/Game/Blueprints/On_Off.WallHited` (`self.Controlled_3`))
  (message `/Game/Blueprints/On_Off.WallHited` (`self.Controlled_4`))
  (message `/Game/Blueprints/On_Off.WallHited` (`self.Controlled_5`)))

(fn `UserConstructionScript`)