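; Fish actor that continuously spins through full pitch revolutions, changing heading after each one.
; Tick sets the root component's world rotation and advances pitch by a fixed step per frame, so spin speed depends on frame rate.
; When pitch completes a full turn it wraps to zero and resets a DoOnce, which picks a random yaw from the Angles array on the next tick.
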(event `self.ReceiveTick`
  (params (DeltaSeconds :type "Float (single-precision)"))
  (bind _rotation (`self.Rotation`))
  (`|ExecutionSequence`
    (:`then_0`
      (`/Engine/EditorBlueprintResources/StandardMacros.DoOnce` false :!label _label
        (:`Completed`
          (set `self.New Angle` (`KismetMathLibrary.Conv_IntToDouble` (`|GetArrayItem` (`self.Angles`) (`KismetMathLibrary.RandomInteger` 4)))))))
    (:`then_1`
      (`SceneComponent.K2_SetWorldRotation` (`self.DefaultSceneRoot`) (`KismetMathLibrary.MakeRotator` 0.0 _rotation (`self.New Angle`)) false false)
      (bind _output_get (set `self.Rotation` (+ _rotation 2.0)))
      (if (== _output_get 360.0)
        (set `self.Rotation` 0.0)
        (goto _label :!via `Reset`)))))

(fn `UserConstructionScript`)