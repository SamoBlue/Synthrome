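; Trap actor that slides between editable start and end offsets using an InterpToMovement component.
; The construction script builds the two relative control points and sets the travel duration from Timer.
; Tick re-rolls Timer and activates the movement after a random latent delay, with a trailing delay that leads nowhere.
; The re-rolled Timer is never written back to the component's Duration at runtime.
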(event `self.ReceiveTick`
  (params (DeltaSeconds :type "Float (single-precision)"))
  (bind _returnvalue (`KismetMathLibrary.RandomFloatInRange` 1.0 7.0))
  (set `self.Timer` _returnvalue)
  (`KismetSystemLibrary.Delay` (`KismetMathLibrary.RandomFloatInRange` 1.0 5.0))
  (`ActorComponent.Activate` (`self.InterpToMovement`) false)
  (`KismetSystemLibrary.Delay` _returnvalue))

(fn `UserConstructionScript`
  (bind _interptomovement (`self.InterpToMovement`))
  (set `InterpToMovementComponent.ControlPoints` (`|MakeArray` (make `InterpControlPoint` (`self.Start Location`)) (make `InterpControlPoint` (`self.End Location`))) _interptomovement)
  (set `InterpToMovementComponent.Duration` (`self.Timer`) _interptomovement))