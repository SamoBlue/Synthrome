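; Drivable Porsche 911 GT3 Chaos wheeled vehicle, controlled by player or AI, with handbrake, traction control and delayed engine start.
; Tick feeds engine audio and, only when player-controlled, mouse steering with velocity-based countersteer blending and camera updates.
; A looping timer drives rear-wheel drift smoke and skid effects, brake and reverse lights, and random chase-camera shake.
; Mouse wheel cycles chase, orbit, cockpit, bumper and fender views with fades.
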(event `self.ReceiveBeginPlay`
  (`KismetSystemLibrary.K2_SetTimerDelegate` (delegate `Timer`) 0.05 true)
  (bind _aschaos_wheeled_vehicle_movement_component (cast `ChaosWheeledVehicleMovementComponent` (`self.VehicleMovementComponent`)))
  (set `self.Movement Component Variable` _aschaos_wheeled_vehicle_movement_component)
  (`KismetSystemLibrary.Delay` 2.0)
  (set `self.Engine Started` true)
  (`self.Traction Control` (`self.TractionControl Enabled`))
  (if (not (`self.IsPlayerControlled`))
    (`SceneComponent.SetVisibility` (`self.SpeedRender`) true true)))

(event `Timer`
  ;[1 1 1] Put these 2 on a timer to improve performance
  (`self.Detect Drift`)
  (`self.Materials Update`)
  (set `self.Chase Camera Shake` (`KismetMathLibrary.MakeVector` (`KismetMathLibrary.RandomFloatInRange` -15.0 20.0) (`KismetMathLibrary.RandomFloatInRange` -20.0 20.0) (`KismetMathLibrary.RandomFloatInRange` -5.0 10.0))))

(event `self.ReceiveTick`
  (params (DeltaSeconds :type "Float (single-precision)"))
  ;[1 1 1] It is better for performance to put as little code as possible on event tick unless absolutely necessary.  Camera movement and receive player inputs has to go here tho.  Also this branch is ensuring the vehicle does not look for inputs if not player controlled, this is vital for the AI to be able to set its inputs.
  (`self.Sounds Inputs`)
  (if (`self.IsPlayerControlled`)
    (`self.Vehicle Input`)
    (`self.Camera Input`)))

(event `Key|MouseScrollUp`
  (params (Key :type "Key Structure"))
  (bind _camera_index (`self.Camera Index`))
  (:`Pressed`
    (set `self.Camera Index` (select `bool` (>= _camera_index 4) :`false` (+ _camera_index 1)))
    (`self.Cycle Cameras` :!label _label)))

(event `Key|MouseScrollDown`
  (params (Key :type "Key Structure"))
  (bind _camera_index (`self.Camera Index`))
  (:`Pressed`
    (set `self.Camera Index` (select `bool` (<= _camera_index 0) :`false` (- _camera_index 1) :`true` 4))
    (goto _label)))

(event `InputAction|Toggle_TC`
  (params (Key :type "Key Structure"))
  (:`Pressed`
    (bind _output_get (set `self.TractionControl Enabled` (not (`self.TractionControl Enabled`))))
    (`self.Traction Control` _output_get)))

(event `InputAction|View_Backward`
  (params (Key :type "Key Structure"))
  (:`Pressed`
    (set `self.Look Back` true))
  (:`Released`
    (set `self.Look Back` false)
    (`SceneComponent.K2_SetRelativeRotation` (`self.SpringArm_Chase`) (struct :`Pitch` -7.0) false false)))

(event `InputAction|Handbrake`
  (params (Key :type "Key Structure"))
  (:`Pressed`
    (`self.Handbrake Toggle` true))
  (:`Released`
    (`self.Handbrake Toggle` false)))

(event `Key|RightMouseButton`
  (params (Key :type "Key Structure"))
  (bind _vehiclemovementcomponent (`self.VehicleMovementComponent`))
  ;[1 1 1] Will refine this in the future but works.
  (:`Pressed`
    (`ChaosVehicleMovementComponent.SetUseAutomaticGears` _vehiclemovementcomponent true)
    (`ChaosVehicleMovementComponent.SetTargetGear` _vehiclemovementcomponent -1 false))
  (:`Released`
    (`ChaosVehicleMovementComponent.SetUseAutomaticGears` _vehiclemovementcomponent true)
    (`ChaosVehicleMovementComponent.SetTargetGear` _vehiclemovementcomponent 1 false)))

(fn `Add Forces`)

(fn `Camera Input`
  (bind _speed (`self.Speed`))
  (bind _springarm_chase (`self.SpringArm_Chase`))
  (bind _springarm_chase_2 (`self.SpringArm_Chase`))
  (bind _camera_chase (`self.Camera_Chase`))
  (bind _mesh (`self.Mesh`))
  (bind (_chase_camera_offset_x _chase_camera_offset_y _chase_camera_offset_z) (`KismetMathLibrary.BreakVector` (`self.Chase Camera Offset`)))
  (bind _springarm_chase_3 (`self.SpringArm_Chase`))
  (bind _springarm_chase_4 (`self.SpringArm_Chase`))
  (bind _camera_cockpit (`self.Camera_Cockpit`))
  (bind _steering_angle (`self.Steering Angle`))
  (bind _camera_cockpit_2 (`self.Camera_Cockpit`))
  (bind (_cockpit_camera_offset_x _cockpit_camera_offset_y _cockpit_camera_offset_z) (`KismetMathLibrary.BreakVector` (`self.Cockpit Camera Offset`)))
  (bind _returnvalue (`SceneComponent.GetComponentVelocity` _mesh))
  (bind _returnvalue_2 (`SceneComponent.K2_GetComponentToWorld` _mesh))
  (bind _relativelocation_x (`KismetMathLibrary.BreakVector` (`SceneComponent.RelativeLocation` _springarm_chase_2)))
  (bind (_relativerotation_roll _relativerotation_pitch _relativerotation_yaw) (`KismetMathLibrary.BreakRotator` (`SceneComponent.RelativeRotation` _springarm_chase_3)))
  (bind (_relativerotation_roll_2 _relativerotation_pitch_2 _relativerotation_yaw_2) (`KismetMathLibrary.BreakRotator` (`SceneComponent.RelativeRotation` _camera_cockpit_2)))
  (bind _relativelocation_x_2 (`KismetMathLibrary.BreakVector` (`SceneComponent.RelativeLocation` _camera_cockpit)))
  (bind (_returnvalue_roll _returnvalue_pitch _returnvalue_yaw) (`KismetMathLibrary.BreakRotator` (`KismetMathLibrary.FindRelativeLookAtRotation` _returnvalue_2 (+ (.location _returnvalue_2) _returnvalue))))
  (switch `int` (`self.Camera Index`)
    (:`0`
      (`CameraComponent.SetFieldOfView` (`self.Camera_Chase`) (`KismetMathLibrary.MapRangeClamped` (`self.Speed`) 0.0 100.0 90.0 120.0))
      (set `SpringArmComponent.TargetArmLength` (`KismetMathLibrary.FInterpTo` (`SpringArmComponent.TargetArmLength` (`self.SpringArm_Chase`)) (`KismetMathLibrary.MapRangeClamped` (`KismetMathLibrary.SelectFloat` (`KismetMathLibrary.Abs` _returnvalue_yaw) 0.0 (and (> (`KismetMathLibrary.VSize` _returnvalue) 500.0) (< _returnvalue_yaw 110.0))) 0.0 45.0 450.0 375.0) (`GameplayStatics.GetWorldDeltaSeconds`) 2.0) _springarm_chase)
      (`SceneComponent.K2_SetRelativeRotation` _springarm_chase (`KismetMathLibrary.SelectRotator` (`KismetMathLibrary.MakeRotator` 0.0 -12.0 180.0) (`KismetMathLibrary.RInterpTo` (`SceneComponent.RelativeRotation` _springarm_chase) (`KismetMathLibrary.MakeRotator` (`KismetMathLibrary.FClamp` (* (`self.Steering Angle`) (`KismetMathLibrary.MapRangeClamped` _speed 5.0 45.0 0.0 0.5)) -10.0 10.0) -9.0 (`KismetMathLibrary.FClamp` (* (`self.Steering Angle`) (`KismetMathLibrary.MapRangeClamped` _speed 5.0 45.0 1.0 0.5)) -45.0 45.0)) (`GameplayStatics.GetWorldDeltaSeconds`) 3.0) (`self.Look Back`)) false false)
      (`SceneComponent.K2_SetRelativeLocation` _springarm_chase_2 (`KismetMathLibrary.MakeVector` (`KismetMathLibrary.FInterpTo` _relativelocation_x (+ (`KismetMathLibrary.Lerp` (`KismetMathLibrary.MapRangeClamped` (`self.Speed`) 0.0 30.0 0.0 50.0) (* (`KismetMathLibrary.SelectFloat` -10.0 -100.0 (== (`ChaosVehicleMovementComponent.GetCurrentGear` (`self.Movement Component Variable`)) 0)) (`KismetMathLibrary.MapRangeClamped` (`self.RPM`) 1000.0 9000.0 0.0 1.0)) (`KismetMathLibrary.MapRangeClamped` (- (`self.GetInputAxisValue`) (`self.GetInputAxisValue`)) -1.0 1.0 0.0 1.0)) _chase_camera_offset_x) (`GameplayStatics.GetWorldDeltaSeconds`) 1.0) _chase_camera_offset_y _chase_camera_offset_z) false false)
      (`SceneComponent.K2_SetRelativeLocation` _camera_chase (`KismetMathLibrary.VInterpTo` (`SceneComponent.RelativeLocation` _camera_chase) (* (`self.Chase Camera Shake`) (`KismetMathLibrary.MapRangeClamped` (`self.Speed`) 5.0 70.0 0.0 1.0)) (`GameplayStatics.GetWorldDeltaSeconds`) (* (`KismetMathLibrary.MapRangeClamped` (`self.Speed`) 5.0 70.0 0.05 3.0) 1.5)) false false))
    (:`1`
      (set `SpringArmComponent.TargetArmLength` 485.0 _springarm_chase_4)
      (`SceneComponent.K2_SetRelativeLocation` _springarm_chase_4 (`self.Orbit Camera Offset`) false false)
      (`SceneComponent.K2_SetRelativeRotation` _springarm_chase_3 (`KismetMathLibrary.MakeRotator` 0.0 (+ _relativerotation_pitch (`self.GetInputAxisValue`)) (+ _relativerotation_yaw (`self.GetInputAxisValue`))) false false)
      (`CameraComponent.SetFieldOfView` (`self.Camera_Chase`) 90.0))
    (:`2`
      (`SceneComponent.K2_SetRelativeRotation` _camera_cockpit_2 (`KismetMathLibrary.MakeRotator` (`KismetMathLibrary.MapRangeClamped` _steering_angle -60.0 60.0 -7.0 7.0) 0.0 (`KismetMathLibrary.FInterpTo` _relativerotation_yaw_2 (* _steering_angle 0.75) (`GameplayStatics.GetWorldDeltaSeconds`) 3.0)) false false)
      (`SceneComponent.K2_SetRelativeLocation` _camera_cockpit (`KismetMathLibrary.MakeVector` (`KismetMathLibrary.FInterpTo` _relativelocation_x_2 (+ (`KismetMathLibrary.Lerp` (`KismetMathLibrary.MapRangeClamped` (`self.Speed`) 0.0 50.0 0.0 10.0) (* (`KismetMathLibrary.SelectFloat` 0.0 -3.0 (== (`ChaosVehicleMovementComponent.GetCurrentGear` (`self.Movement Component Variable`)) 0)) (`KismetMathLibrary.MapRangeClamped` (`self.RPM`) 1000.0 9000.0 0.0 1.0)) (`KismetMathLibrary.MapRangeClamped` (- (`self.GetInputAxisValue`) (`self.GetInputAxisValue`)) -1.0 1.0 0.0 1.0)) _cockpit_camera_offset_x) (`GameplayStatics.GetWorldDeltaSeconds`) 7.0) _cockpit_camera_offset_y _cockpit_camera_offset_z) false false))))

(fn `Cycle Cameras`
  (bind _camera_chase (`self.Camera_Chase`))
  (bind _returnvalue (select `int` (`self.Camera Index`) :`0` _camera_chase :`1` _camera_chase :`2` (`self.Camera_Cockpit`) :`3` (`self.Camera_Bumper`) :`4` (`self.Camera_Fender`) :!type "SceneComponent Object Reference"))
  (`PlayerCameraManager.StartCameraFade` :`self` (`PlayerController.PlayerCameraManager` (`GameplayStatics.GetPlayerController` 0)) :`ToAlpha` 1.0 :`Duration` 0.5 :`bShouldFadeAudio` true)
  (`ActorComponent.SetActive` (`self.Camera_Cockpit`) false false)
  (`ActorComponent.SetActive` (`self.Camera_Bumper`) false false)
  (`ActorComponent.SetActive` (`self.Camera_Fender`) false false)
  (`ActorComponent.SetActive` (`self.Camera_Chase`) false false)
  (`SceneComponent.SetVisibility` (`self.Camera_Chase`) false true)
  (`SceneComponent.SetVisibility` (`self.Camera_Cockpit`) false true)
  (`SceneComponent.SetVisibility` (`self.Camera_Bumper`) false true)
  (`SceneComponent.SetVisibility` (`self.Camera_Fender`) false true)
  (`ActorComponent.SetActive` _returnvalue true false)
  (`SceneComponent.SetVisibility` _returnvalue true true)
  (`PlayerCameraManager.StartCameraFade` :`self` (`PlayerController.PlayerCameraManager` (`GameplayStatics.GetPlayerController` 0)) :`FromAlpha` 1.0 :`Duration` 1.0 :`bShouldFadeAudio` true))

(fn `Detect Drift`
  (bind _movement_component_variable (`self.Movement Component Variable`))
  (set `self.Is Drifting` false)
  (for (_array_element _array_index) (`ChaosWheeledVehicleMovementComponent.Wheels` _movement_component_variable)
    (if (`KismetMathLibrary.InRange_IntInt` _array_index 2 3)
      (bind (_bincontact _contactpoint _physmaterial _normalizedsuspensionlength _springforce _slipangle _bisslipping _slipmagnitude _bisskidding _skidmagnitude) (`ChaosWheeledVehicleMovementComponent.BreakWheelStatus` (`ChaosWheeledVehicleMovementComponent.GetWheelState` _movement_component_variable _array_index)))
      (if (and (not (`ChaosVehicleWheel.IsInAir` _array_element)) (or _bisslipping _bisskidding))
        (set `self.Is Drifting` true)
        (bind _output (`|GetArrayItem` (`self.Skid Emmiters`) _array_index))
        (if (== _output null)
          (bind _returnvalue (`NiagaraFunctionLibrary.SpawnSystemAttached` "/Game/Vehicles/00_Common/FX/PS_Drift_Asphalt.PS_Drift_Asphalt" (select `int` _array_index :`0` null :`1` null :`2` (`self.Wheel_RL`) :`3` (`self.Wheel_RR`)) "None" (0.0 0.0 0.0) (struct) "KeepRelativeOffset"))
          (`NiagaraComponent.SetVariableFloat` _returnvalue "SmokeAmmount" (`KismetMathLibrary.SignOfFloat` _slipmagnitude))
          (`KismetArrayLibrary.Array_Set` (`self.Skid Emmiters`) _array_index _returnvalue)
          (else
            (`NiagaraComponent.SetVariableFloat` _output "SmokeAmmount" (`KismetMathLibrary.SignOfFloat` _slipmagnitude))
            (`NiagaraComponent.SetVariableFloat` _output "SkidOpacity" (`KismetMathLibrary.FClamp` (+ (`KismetMathLibrary.MapRangeClamped` (`KismetMathLibrary.Abs` _slipmagnitude) 600.0 1000.0 0.0 1.0) (`KismetMathLibrary.MapRangeClamped` (`KismetMathLibrary.Abs` _skidmagnitude) 1000.0 1500.0 0.0 1.0))))))
        (else
          (bind _output_2 (`|GetArrayItem` (`self.Skid Emmiters`) _array_index))
          (if (not (== _output_2 null))
            (`NiagaraComponent.SetVariableFloat` _output_2 "SmokeAmmount" 0.0)
            (`SceneComponent.K2_DetachFromComponent` _output_2 "KeepWorld" "KeepWorld" "KeepWorld" true)
            (`KismetArrayLibrary.Array_Set` (`self.Skid Emmiters`) _array_index)))))))

(fn `Handbrake Toggle`
  (params (Handbrake :type Boolean))
  (bind _vehiclemovementcomponent (`self.VehicleMovementComponent`))
  (if Handbrake
    (set `self.Gear Before Handbrake` (`ChaosVehicleMovementComponent.GetCurrentGear` _vehiclemovementcomponent))
    (`ChaosVehicleMovementComponent.SetTargetGear` _vehiclemovementcomponent 0 true)
    (`ChaosVehicleMovementComponent.SetHandbrakeInput` _vehiclemovementcomponent true)
    (`ChaosVehicleMovementComponent.SetUseAutomaticGears` _vehiclemovementcomponent false)
    (else
      (`ChaosVehicleMovementComponent.SetTargetGear` _vehiclemovementcomponent (`KismetMathLibrary.SelectInt` (`self.Gear Before Handbrake`) 1 (`self.Is Drifting`)) true)
      (`ChaosVehicleMovementComponent.SetHandbrakeInput` _vehiclemovementcomponent false)
      (`ChaosVehicleMovementComponent.SetUseAutomaticGears` _vehiclemovementcomponent true))))

(fn `Materials Update`
  (bind _mesh (`self.Mesh`))
  (bind _mesh_2 (`self.Mesh`))
  (bind _returnvalue (`MeshComponent.GetMaterialIndex` _mesh "ReverseLight"))
  (bind _returnvalue_2 (`MeshComponent.GetMaterialIndex` _mesh_2 "BrakeLight"))
  (bind _returnvalue_3 (`PrimitiveComponent.CreateDynamicMaterialInstance` _mesh_2 _returnvalue_2 (`PrimitiveComponent.GetMaterial` _mesh_2 _returnvalue_2) "None"))
  (`MaterialInstanceDynamic.SetScalarParameterValue` _returnvalue_3 "Facing Intensity (cd/m2)" (`KismetMathLibrary.Lerp` 0.5 15.0 (`self.GetInputAxisValue`)))
  (bind _returnvalue_4 (`PrimitiveComponent.CreateDynamicMaterialInstance` _mesh _returnvalue (`PrimitiveComponent.GetMaterial` _mesh _returnvalue) "None"))
  (`MaterialInstanceDynamic.SetScalarParameterValue` _returnvalue_4 "Facing Intensity (cd/m2)" (`KismetMathLibrary.SelectFloat` 10.0 0.0 (== (`ChaosVehicleMovementComponent.GetCurrentGear` (`self.Movement Component Variable`)) -1))))

(fn `Sounds Inputs`
  (`AudioParameterControllerInterface.SetFloatParameter` (`self.SFX_Engine`) "RPM Range" (`KismetMathLibrary.MapRangeClamped` (`ChaosWheeledVehicleMovementComponent.GetEngineRotationSpeed` (`self.Movement Component Variable`)) 1000.0 9000.0 0.0 1.0))
  (`AudioParameterControllerInterface.SetFloatParameter` (`self.SFX_Engine`) "Load Multiplier" (`KismetMathLibrary.MapRangeClamped` (- (`self.RPM`) (`self.Last RPM`)) -30.0 10.0 0.0 1.0)))

(fn `Traction Control`
  (params (InputPin :type Boolean))
  (bind _movement_component_variable (`self.Movement Component Variable`))
  (for (_ _array_index) (`ChaosWheeledVehicleMovementComponent.Wheels` _movement_component_variable)
    (`ChaosWheeledVehicleMovementComponent.SetTractionControlEnabled` _movement_component_variable _array_index InputPin)))

(fn `UserConstructionScript`
  (bind (_color_r _color_g _color_b) (break `LinearColor` (`self.Color`)))
  (set `self.Tags` (`|MakeArray` (`self.Name`)))
  (if (`self.Use Custom Color`)
    (`TextRenderComponent.SetTextRenderColor` (`self.NameRender`) (`KismetMathLibrary.Conv_LinearColorToColor` (make `LinearColor` _color_r _color_g _color_b 0.1)))))

(fn `Vehicle Input`
  (bind _returnvalue (`self.GetTransform`))
  (bind _vehiclemovementcomponent (`self.VehicleMovementComponent`))
  (bind _movement_component_variable (`self.Movement Component Variable`))
  (bind _returnvalue_2 (`ChaosVehicleMovementComponent.GetForwardSpeedMPH` (`self.Movement Component Variable`)))
  (bind _returnvalue_3 (`SceneComponent.GetComponentVelocity` (`self.Mesh`)))
  (bind (_returnvalue_roll _returnvalue_pitch _returnvalue_yaw) (`KismetMathLibrary.BreakRotator` (`KismetMathLibrary.FindRelativeLookAtRotation` _returnvalue (+ (.location _returnvalue) _returnvalue_3))))
  (bind _returnvalue_4 (`KismetMathLibrary.Abs` _returnvalue_yaw))
  (bind _returnvalue_5 (* _returnvalue_yaw 1.5))
  (bind _returnvalue_6 (`KismetMathLibrary.MapRangeClamped` (`KismetMathLibrary.SelectFloat` _returnvalue_4 0.0 (and (> (`KismetMathLibrary.VSize` _returnvalue_3) 500.0) (< _returnvalue_4 110.0))) 5.0 50.0 0.0 1.0))
  (bind _returnvalue_7 (`KismetMathLibrary.Lerp` (* (`KismetMathLibrary.FClamp` (+ (`self.Steering Angle`) (* (`self.GetInputAxisValue`) (`KismetMathLibrary.MapRangeClamped` _returnvalue_2 0.0 90.0 1.0 0.6))) -70.0 70.0) (`KismetMathLibrary.MapRangeClamped` _returnvalue_2 60.0 110.0 1.0 0.99)) _returnvalue_5 _returnvalue_6))
  ;[1 1 1] Just your basic input setup,  using the axis values instead of events to keep the graph clean
  (`ChaosVehicleMovementComponent.SetThrottleInput` _vehiclemovementcomponent (`KismetMathLibrary.SelectFloat` (`self.GetInputAxisValue`) 0.0 (`self.Engine Started`)))
  (`ChaosVehicleMovementComponent.SetBrakeInput` _vehiclemovementcomponent (`self.GetInputAxisValue`))
  (if (== (`self.Camera Index`) 1)
    (`ChaosVehicleMovementComponent.SetSteeringInput` _vehiclemovementcomponent (`KismetMathLibrary.Lerp` (`self.GetInputAxisValue`) (`KismetMathLibrary.MapRangeClamped` _returnvalue_5 -70.0 70.0 -1.0 1.0) _returnvalue_6))
    (else
      ;[1 1 1] Using mouse input for steering the vehicle.
      (set `self.Steering Angle` _returnvalue_7)
      (`ChaosVehicleMovementComponent.SetSteeringInput` _vehiclemovementcomponent (`KismetMathLibrary.MapRangeClamped` _returnvalue_7 -70.0 70.0 -1.0 1.0))))
  ;[1 1 1] Setting variables for things we are going to use alot, all over the graph.
  (set `self.Speed` (`KismetMathLibrary.Abs` (`ChaosVehicleMovementComponent.GetForwardSpeedMPH` _movement_component_variable)))
  (set `self.Last RPM` (`self.RPM`))
  (set `self.RPM` (`ChaosWheeledVehicleMovementComponent.GetEngineRotationSpeed` _movement_component_variable)))