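; Drivable Nissan Skyline R34 vehicle Blueprint that builds on a parent class for its BeginPlay, Tick and construction logic.
; E and Q shift the movement component's target gear up and down, clamped from reverse to fifth.
; The construction script optionally applies a custom color through a dynamic instance of the Paint material.
; An unconnected, never-run graph would lower friction on wheels 2 and 3 as slip angle grows.
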(event `self.ReceiveBeginPlay`
  (`parent.ReceiveBeginPlay`))

(event `self.ReceiveTick`
  (params (DeltaSeconds :type "Float (single-precision)"))
  (`parent.ReceiveTick` DeltaSeconds))

(event `Key|E`
  (params (Key :type "Key Structure"))
  (bind _vehiclemovementcomponent (`self.VehicleMovementComponent`))
  (:`Pressed`
    (`ChaosVehicleMovementComponent.SetTargetGear` _vehiclemovementcomponent (`KismetMathLibrary.Clamp` (+ (`ChaosVehicleMovementComponent.GetCurrentGear` _vehiclemovementcomponent) 1) -1 5) false)))

(event `Key|Q`
  (params (Key :type "Key Structure"))
  (:`Pressed`
    (`ChaosVehicleMovementComponent.SetTargetGear` (`self.VehicleMovementComponent`) (`KismetMathLibrary.Clamp` (- (`ChaosVehicleMovementComponent.GetCurrentGear` (`self.VehicleMovementComponent`)) 1) -1 5) false)))

(fn `UserConstructionScript`
  (bind _mesh (`self.Mesh`))
  (bind _returnvalue (`MeshComponent.GetMaterialIndex` _mesh "Paint"))
  (`parent.UserConstructionScript`)
  (if (`self.Use Custom Color`)
    (bind _returnvalue_2 (`PrimitiveComponent.CreateDynamicMaterialInstance` _mesh _returnvalue (`PrimitiveComponent.GetMaterial` _mesh _returnvalue) "None"))
    (`MaterialInstanceDynamic.SetVectorParameterValue` _returnvalue_2 "Color" (`self.Color`))))