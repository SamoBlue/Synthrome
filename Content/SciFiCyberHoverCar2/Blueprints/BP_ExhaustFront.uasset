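; BP_ExhaustFront is a front exhaust effect for a sci-fi hover car, made of an exhaust mesh and a looping-style exhaust sound driven by engine power.
; CalculateEnginePower smooths the absolute engine power with FInterpTo and feeds it, clamped, to the mesh material's EnginePower parameter.
; Tick sets the sound's Volume parameter from that smoothed power plus a parking offset, capped low.
; SetExhaustColor tints the mesh material.
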(event `self.ReceiveTick`
  (params (DeltaSeconds :type "Float (single-precision)"))
  ;[1 1 1] Sounds Control
  (`AudioComponent.SetFloatParameter` (`self.ExhaustSound`) "Volume" (`KismetMathLibrary.FClamp` (+ (`self.EnginePowerInterpolated`) (`self.ParkingExhaustVolume`)) 0.0 0.2)))

(event `SetExhaustColor`
  (params (InLinearColor :type "LinearColor Structure" :default (struct :`G` 0.658814 :`B` 1.0 :`A` 1.0)))
  ;[1 1 1] Set ExhaustColor
  (`MeshComponent.SetVectorParameterValueOnMaterials` (`self.ExhaustMesh`) "Color" (`KismetMathLibrary.Conv_LinearColorToVector` InLinearColor)))

(event `CalculateEnginePower`
  (params (EnginePower :type "Float (double-precision)") (Min :type "Float (double-precision)" :default 0.5) (Max :type "Float (double-precision)" :default 1.0))
  ;[1 1 1] CalculateEnginePower
  (bind _output_get (set `self.EnginePowerInterpolated` (`KismetMathLibrary.FInterpTo` (`self.EnginePowerInterpolated`) (`KismetMathLibrary.Abs` EnginePower) (`GameplayStatics.GetWorldDeltaSeconds`) (`self.InterpolationSpeed`))))
  (`MeshComponent.SetScalarParameterValueOnMaterials` (`self.ExhaustMesh`) "EnginePower" (`KismetMathLibrary.FClamp` _output_get Min Max)))

(fn `UserConstructionScript`)